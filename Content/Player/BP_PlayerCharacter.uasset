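; Player character Blueprint that implements a blade barrage super: a physics leap followed by a blade spawn.
; BeginPlay registers the Enhanced Input mapping context, and the Super action sets a HasSupered flag while adding upward velocity to PlayerBody.
; Tick watches for vertical velocity to reach zero or below, then spawns BP_BladeBarrageBlade at an offset from the forward vector and clears the flag.
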(event Input|EnhancedActionEvents|EnhancedInputActionIA_Super
  (params (ActionValue :type Boolean) (ElapsedSeconds :type Float%20%28double-precision%29) (TriggeredSeconds :type Float%20%28double-precision%29) (InputAction :type Input%20Action%20Object%20Reference :default "/Game/Player/IA_Super.IA_Super"))
  (:Started
    (if (not (Variables|Default|GetHasSupered))
      (Variables|Default|SetHasSupered true)
      (Development|PrintString "Super Cast")
      (Physics|SetPhysicsLinearVelocity (Variables|Default|GetPlayerBody) (Math|Vector|MakeVector 0.0 0.0 (Math|Conversions|ToFloat(Integer) (Variables|Default|GetJumpForce))) true "None"))))

(event EventBeginPlay
  (bind _returnvalue (Class|InputDeviceLibrary|GetPlayerControllerfromInputDevice))
  (Input|AddMappingContext (PlayerController|LocalPlayerSubsystems|GetEnhancedInputLocalPlayerSubsystem _returnvalue) "/Game/Player/IMC_PlayerInput.IMC_PlayerInput" 0 "(bIgnoreAllPressedKeysUntilRelease=True,bForceImmediately=False,bNotifyUserSettings=False)"))

(event Collision|EventActorBeginOverlap
  (params (OtherActor :type Actor%20Object%20Reference)))

(event EventTick
  (params (DeltaSeconds :type Float%20%28single-precision%29))
  (if (Variables|Default|GetHasSupered)
    (bind _returnvalue (Physics|GetPhysicsLinearVelocity (Variables|Default|GetPlayerBody) "None"))
    (if (<= (.z _returnvalue) 0.0)
      (Game|SpawnActorfromClass "/Game/BP_BladeBarrageBlade.BP_BladeBarrageBlade_C" (Math|Conversions|ToTransform(Vector) (+ (* (Math|Vector|GetForwardVector (Variables|Default|GetPlayerBody)) "500.000000,1.000000,1.000000") (Transformation|GetActorLocation))) "Undefined" "MultiplyWithRoot" 0 0)
      (Development|PrintString "Blades Spawned")
      (Variables|Default|SetHasSupered false))))

(fn ConstructionScript)
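; BP_Player is a player character with a castable super and 90-degree left/right turning through Enhanced Input, with its class set to Solar at start.
; The super input launches the character upward, then Tick waits for downward capsule velocity to trigger Blade Barrage.
; The barrage spawns a row of blade actors along a fixed world axis ahead of the player, adds forward-based velocity to each and clears the super flag.
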(event Input|EnhancedActionEvents|EnhancedInputActionIA_Super
  (params (ActionValue :type Boolean) (ElapsedSeconds :type Float%20%28double-precision%29) (TriggeredSeconds :type Float%20%28double-precision%29) (InputAction :type Input%20Action%20Object%20Reference :default "/Game/Player/Input/IA_Super.IA_Super"))
  (:Started
    (if (not (Variables|Default|GetHasSupered))
      (Character|LaunchCharacter (Math|Vector|MakeVector 0.0 0.0 (Math|Conversions|ToFloat(Integer) (Variables|Default|GetJumpForce))) false false)
      (Variables|Default|SetHasSupered true)
      (Development|PrintString "Super Cast"))))

(event Input|EnhancedActionEvents|EnhancedInputActionIA_RotateLeft
  (params (ActionValue :type Boolean) (ElapsedSeconds :type Float%20%28double-precision%29) (TriggeredSeconds :type Float%20%28double-precision%29) (InputAction :type Input%20Action%20Object%20Reference :default "/Game/Player/Input/IA_RotateLeft.IA_RotateLeft"))
  (bind _returnvalue (Transformation|GetActorRotation))
  (:Started
    (Transformation|SetActorRotation (Math|Rotator|MakeRotator (.roll _returnvalue) (.pitch _returnvalue) (+ (.yaw _returnvalue) -9e+01)))
    (Development|PrintString "Left Rotated")))

(event Input|EnhancedActionEvents|EnhancedInputActionIA_RotateRight
  (params (ActionValue :type Boolean) (ElapsedSeconds :type Float%20%28double-precision%29) (TriggeredSeconds :type Float%20%28double-precision%29) (InputAction :type Input%20Action%20Object%20Reference :default "/Game/Player/Input/IA_RotateRight.IA_RotateRight"))
  (bind _returnvalue (Transformation|GetActorRotation))
  (:Started
    (Transformation|SetActorRotation (Math|Rotator|MakeRotator (.roll _returnvalue) (.pitch _returnvalue) (+ (.yaw _returnvalue) 9e+01)))
    (Development|PrintString "Right Rotated")))

(event EventBeginPlay
  (bind _returnvalue (Class|InputDeviceLibrary|GetPlayerControllerfromInputDevice))
  (Input|AddMappingContext (PlayerController|LocalPlayerSubsystems|GetEnhancedInputLocalPlayerSubsystem _returnvalue) "/Game/Player/Input/IMC_PlayerInput.IMC_PlayerInput" 0 "(bIgnoreAllPressedKeysUntilRelease=True,bForceImmediately=False,bNotifyUserSettings=False)")
  (Variables|Default|SetClass "NewEnumerator0"))

(event Collision|EventActorBeginOverlap
  (params (OtherActor :type Actor%20Object%20Reference)))

(event EventTick
  (params (DeltaSeconds :type Float%20%28single-precision%29))
  (if (Variables|Default|GetHasSupered)
    (bind _returnvalue (Physics|GetPhysicsLinearVelocity (Variables|Collision|GetCapsuleComponent) "None"))
    (if (<= (.z _returnvalue) -1.0)
      (switch Utilities|FlowControl|Switch|SwitchonPlayerSubclass (Variables|Default|GetClass)
        (:NewEnumerator0
          (CallFunction|ActivateBladeBarrage))))))

(fn ConstructionScript)

(fn ActivateBladeBarrage
  (bind _bladestospawn (Variables|Default|GetbladesToSpawn))
  (bind _capsulecomponent (Variables|Collision|GetCapsuleComponent))
  (bind _returnvalue (Math|Vector|GetForwardVector _capsulecomponent))
  (for _index (range 0 (- _bladestospawn 1))
    (bind _returnvalue_2 (Game|SpawnActorfromClass "/Game/BP_BladeBarrageBlade.BP_BladeBarrageBlade_C" (Math|Conversions|ToTransform(Vector) (+ (* (Math|Vector|GetRightVector "0, 0, 0") (* (- _index 1) (/ (Variables|Default|GetbladesLineLength) (- _bladestospawn 1)))) (+ (* _returnvalue "500.000000,1.000000,1.000000") (Transformation|GetActorLocation)))) "Undefined" "MultiplyWithRoot" 0 0))
    (Physics|SetPhysicsLinearVelocity (Variables|/Game/BP_BladeBarrageBlade.BP_BladeBarrageBlade_C|GetCube _returnvalue_2) (* _returnvalue "2000.000000,1.000000,1.000000") true "None")
    (Variables|Default|SetHasSupered false)))